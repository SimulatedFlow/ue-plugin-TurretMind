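; BP_TurretMindDemoDirector runs a TurretMind demo, managing the population of walker actors and enabling stats and range drawing on BeginPlay, with debug drawing off.
; A looping timer calls AdjustPopulation, which spawns walkers at the world origin or destroys the newest ones until the array matches DesiredCount.
; Wave events switch DesiredCount between a small and a large crowd, leaving the timer to apply the change.
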(event Custom|AdjustPopulation
  (bind _returnvalue (Class|KismetSystemLibrary|MakeLiteralInteger 1))
  (bind _walkers (Variables|Default|GetWalkers))
  (bind _returnvalue_2 (Utilities|Array|Length _walkers))
  (bind _returnvalue_3 (- _returnvalue_2 _returnvalue))
  (while (< (Utilities|Array|Length (Variables|Default|GetWalkers)) (Variables|Default|GetDesiredCount))
    (bind _returnvalue_4 (Game|SpawnActorfromClass "/TurretMind/TurretMind/Blueprints/BP_TurretMindWalker.BP_TurretMindWalker_C" (Math|Transform|MakeTransform (Math|Vector|MakeVector 0.0 0.0 0.0)) "AlwaysSpawn" "MultiplyWithRoot" 0 0))
    (Utilities|Array|Add (Variables|Default|GetWalkers) _returnvalue_4))
  (while (> (Utilities|Array|Length (Variables|Default|GetWalkers)) (Variables|Default|GetDesiredCount))
    (Actor|DestroyActor (Utilities|Array|Get(acopy) (Variables|Default|GetWalkers) _returnvalue_3))
    (Utilities|Array|RemoveIndex (Variables|Default|GetWalkers) _returnvalue_3)))

(event Custom|SetWave50
  (Variables|Default|SetDesiredCount 50))

(event Custom|SetWave200
  (Variables|Default|SetDesiredCount 200))

(event EventBeginPlay
  (Class|TurretMindStatics|SetShowStats true)
  (Class|TurretMindStatics|SetDrawRanges true)
  (Class|TurretMindStatics|SetDrawDebug false)
  (Utilities|Time|SetTimerbyFunctionName self "AdjustPopulation" 0.25 true false 0.1))

(event Collision|EventActorBeginOverlap
  (params (OtherActor :type Actor%20Object%20Reference)))

(event EventTick
  (params (DeltaSeconds :type Float%20%28single-precision%29)))

(fn ConstructionScript)